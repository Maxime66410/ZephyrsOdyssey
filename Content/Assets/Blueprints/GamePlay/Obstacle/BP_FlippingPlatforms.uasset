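; BP_FlippingPlatforms is an obstacle platform that flips each time the player jumps.
; A looping 0.01-second timer polls BP_Player's IsJump flag, with a latch allowing one flip attempt per jump.
; CallUpdate alternately plays and reverses the RotateRamp timeline, rolling the Pivot at SpeedMove rate and gated by an animation-done flag.
; GetPlayer caches the player reference and can restart the polling timer, with a capped retry counter.
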(event Custom|CallUpdate
  ;[1 0.1355 0] Call Update PlateForm Rotation
  (if (Variables|State|GetFlipDoneAnimation)
    (if (Variables|State|GetIsFlip?)
      (Variables|State|SetIsFlip? false)
      (bind _floatrotation (Timeline|RotateRamp Play)
        (:Update
          (Transformation|SetRelativeRotation (Variables|Default|GetPivot) (Math|Rotator|MakeRotator _floatrotation 0.0 0.0) false false)
          (Variables|State|SetFlipDoneAnimation false))
        (:Finished
          (Variables|State|SetFlipDoneAnimation true)))
      (else
        (Variables|State|SetIsFlip? true)
        (Timeline|RotateRamp Reverse)))))

(event EventBeginPlay
  ;[0.6259 0.3914 1] Init Flipping Platforms
  (CallFunction|GetPlayer)
  (bind _returnvalue (Utilities|Time|SetTimerbyFunctionName 0 "CheckPlayerJump" 0.01 true))
  (Variables|Event|SetEvent_CheckPlayer _returnvalue)
  (Components|Timeline|SetPlayRate (Variables|Default|GetRotateRamp) (Variables|State|GetSpeedMove)))

(fn ConstructionScript)

(fn GetPlayer
  ;[1 0.3076 0.8269] Check if ref exist
  (Variables|REF|GetPlayerREF
    (:then
      ;[1 0.2891 0.9425] Relauch Event with contraints debug
      (if (!= (Variables|Debug|GetTryingToGetPlayerCount) 10000)
        (if (not (Class|KismetSystemLibrary|TimerExistsHandle (Variables|Event|GetEvent_CheckPlayer)))
          (bind _returnvalue (Utilities|Time|SetTimerbyFunctionName 0 "CheckPlayerJump" 0.01 true))
          (Variables|Event|SetEvent_CheckPlayer _returnvalue)
          (Math|Integer|IncrementInt (Variables|Debug|GetTryingToGetPlayerCount)))))
    (:else
      ;[1 0.7061 0.1344] Get Player
      (bind _asbp_player (Utilities|Casting|CastToBP_Player (Game|GetPlayerCharacter 0)))
      (Variables|REF|SetPlayerREF _asbp_player)
      ;;[0 0 0] Relauch Event
      (CallFunction|GetPlayer))))

(fn CheckPlayerJump
  ;[1 0.2287 0.4405] Check if REF exist
  (Variables|REF|GetPlayerREF
    (:then
      ;[0.2314 0.6597 1] Check if player jump
      (if (Variables|/Game/Assets/Blueprints/Player/BP_Player.BP_Player_C|GetIsJump? (Variables|REF|GetPlayerREF))
        ;[0.1101 1 0.4313] Check is flip is done
        (if (not (Variables|State|GetFlipDone))
          ;[0.9072 0.4696 1] Call Update Rotation
          (CallFunction|CallUpdate)
          ;[1 0.9221 0.4062] Set is flip done
          (Variables|State|SetFlipDone true))
        (else
          (Variables|State|SetFlipDone false))))
    (:else
      ;[0.9124 1 0] Clear & Call get Player
      (CallFunction|GetPlayer)
      (Utilities|Time|ClearandInvalidateTimerbyHandle (Variables|Event|GetEvent_CheckPlayer)))))