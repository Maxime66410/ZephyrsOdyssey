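; BP_Garden is a decorative garden that fills its spawn points with plants when the construction script runs.
; The script resets four instanced mesh components, assigns their meshes from PlantList, then spawns by PlantType: random mix, potato, bush or flowers.
; Each spawn point has a random chance of receiving a plant.
; Per-instance random custom data feeds a shared random-color material, varying plants without separate materials.
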(fn ConstructionScript
  (bind _plantlist (Variables|Default|GetPlantList))
  (Utilities|FlowControl|Sequence
    (:then_0
      (Components|InstancedStaticMesh|ClearInstances (Variables|Default|GetPatatoInstanced))
      (Components|InstancedStaticMesh|ClearInstances (Variables|Default|GetBushInstanced))
      (Components|InstancedStaticMesh|ClearInstances (Variables|Default|GetFlowerInstanced))
      (Components|InstancedStaticMesh|ClearInstances (Variables|Default|GetFlower2Instanced)))
    (:then_1
      (Components|StaticMesh|SetStaticMesh (Variables|Default|GetPatatoInstanced) (Utilities|Array|Get(acopy) _plantlist 1))
      (Components|StaticMesh|SetStaticMesh (Variables|Default|GetBushInstanced) (Utilities|Array|Get(acopy) _plantlist))
      (Components|StaticMesh|SetStaticMesh (Variables|Default|GetFlowerInstanced) (Utilities|Array|Get(acopy) _plantlist 2))
      (Components|StaticMesh|SetStaticMesh (Variables|Default|GetFlower2Instanced) (Utilities|Array|Get(acopy) _plantlist 3)))
    (:then_2
      (Rendering|Material|SetMaterial (Variables|Default|GetPatatoInstanced) 0 "/Game/Assets/Materials/Surface/M_Plants_RandomColor_Inst.M_Plants_RandomColor_Inst")
      (Rendering|Material|SetMaterial (Variables|Default|GetBushInstanced) 0 "/Game/Assets/Materials/Surface/M_Plants_RandomColor_Inst.M_Plants_RandomColor_Inst")
      (Rendering|Material|SetMaterial (Variables|Default|GetFlowerInstanced) 0 "/Game/Assets/Materials/Surface/M_Plants_RandomColor_Inst.M_Plants_RandomColor_Inst")
      (Rendering|Material|SetMaterial (Variables|Default|GetFlower2Instanced) 0 "/Game/Assets/Materials/Surface/M_Plants_RandomColor_Inst.M_Plants_RandomColor_Inst"))
    (:then_3
      (switch Utilities|FlowControl|Switch|SwitchonEPlantType (Variables|Default|GetPlantType)
        (:NewEnumerator1
          (CallFunction|RandomSpawn))
        (:NewEnumerator2
          (CallFunction|PotatoSpawn))
        (:NewEnumerator3
          (CallFunction|BushSpawn))
        (:NewEnumerator4
          (CallFunction|FlowerSpawn))))))

(fn RandomSpawn
  (for _array_element (Utilities|SpawnPosition)
    (LocalVariables|SetRandomPos (Math|Random|RandomBool))
    (LocalVariables|SetRandomPlant (Math|Random|RandomIntegerinRange 0 3))
    (if (LocalVariables|GetRandomPos)
      (bind _returnvalue (Components|InstancedStaticMesh|AddInstance (Utilities|Select :Index (LocalVariables|GetRandomPlant) :Option%200 (Variables|Default|GetPatatoInstanced) :Option%201 (Variables|Default|GetBushInstanced) :Option%202 (Variables|Default|GetFlowerInstanced) :Option%203 (Variables|Default|GetFlower2Instanced)) (Math|Transform|MakeTransform (Transformation|GetWorldLocation _array_element) "0, 0, 0" "1.000000,1.000000,1.000000") true))
      (Components|InstancedStaticMesh|SetCustomDataValue (Utilities|Select :Index (LocalVariables|GetRandomPlant) :Option%200 (Variables|Default|GetPatatoInstanced) :Option%201 (Variables|Default|GetBushInstanced) :Option%202 (Variables|Default|GetFlowerInstanced) :Option%203 (Variables|Default|GetFlower2Instanced)) _returnvalue 0 (Math|Random|RandomFloatinRange 0.1 5.0) false))))

(fn PotatoSpawn
  (bind _patatoinstanced (Variables|Default|GetPatatoInstanced))
  (for _array_element (Utilities|SpawnPosition)
    (LocalVariables|SetRandomPos (Math|Random|RandomBool))
    (if (LocalVariables|GetRandomPos)
      (bind _returnvalue (Components|InstancedStaticMesh|AddInstance _patatoinstanced (Math|Transform|MakeTransform (Transformation|GetWorldLocation _array_element) "0, 0, 0" "1.000000,1.000000,1.000000") true))
      (Components|InstancedStaticMesh|SetCustomDataValue _patatoinstanced _returnvalue 0 (Math|Random|RandomFloatinRange 0.1 3.0) false))))

(fn BushSpawn
  (bind _bushinstanced (Variables|Default|GetBushInstanced))
  (for _array_element (Utilities|SpawnPosition)
    (LocalVariables|SetRandomPos (Math|Random|RandomBool))
    (if (LocalVariables|GetRandomPos)
      (bind _returnvalue (Components|InstancedStaticMesh|AddInstance _bushinstanced (Math|Transform|MakeTransform (Transformation|GetWorldLocation _array_element) "0, 0, 0" "1.000000,1.000000,1.000000") true))
      (Components|InstancedStaticMesh|SetCustomDataValue _bushinstanced _returnvalue 0 (Math|Random|RandomFloatinRange 0.1 2.0) false))))

(fn FlowerSpawn
  (for _array_element (Utilities|SpawnPosition)
    (LocalVariables|SetRandomPos (Math|Random|RandomBool))
    (LocalVariables|SetRandomPlant (Math|Random|RandomIntegerinRange 0 1))
    (if (LocalVariables|GetRandomPos)
      (bind _returnvalue (Components|InstancedStaticMesh|AddInstance (Utilities|Select :Index (LocalVariables|GetRandomPlant) :Option%200 (Variables|Default|GetFlowerInstanced) :Option%201 (Variables|Default|GetFlower2Instanced)) (Math|Transform|MakeTransform (Transformation|GetWorldLocation _array_element) "0, 0, 0" "1.000000,1.000000,1.000000") true))
      (Components|InstancedStaticMesh|SetCustomDataValue (Utilities|Select :Index (LocalVariables|GetRandomPlant) :Option%200 (Variables|Default|GetFlowerInstanced) :Option%201 (Variables|Default|GetFlower2Instanced)) _returnvalue 0 (Math|Random|RandomFloatinRange 1.0 2.0) false))))