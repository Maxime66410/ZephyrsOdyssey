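; BP_CollectibleMaster is a pickup actor whose collectible type selects a coin, star coin or ruby variant.
; The construction script sets the static mesh from that type.
; When BP_Player overlaps the Box, type-based Selects set the score and coins added through GMB_InGame and the 2D sound played.
; It then triggers feedback on the player and destroys itself.
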(event OnComponentBeginOverlap(Box)
  (params (OverlappedComponent :type Primitive%20Component%20Object%20Reference) (OtherActor :type Actor%20Object%20Reference) (OtherComp :type Primitive%20Component%20Object%20Reference) (OtherBodyIndex :type Integer) (bFromSweep :type Boolean) (SweepResult :type Hit%20Result%20Structure%20%28by%20ref%29))
  (bind _ecollectibletype (Variables|Default|GetECollectibleType))
  (bind _asbp_player (Utilities|Casting|CastToBP_Player OtherActor))
  (Variables|Default|SetAs%20BP%20Player _asbp_player)
  (bind _asgmb_in_game (Utilities|Casting|CastToGMB_InGame (Game|GetGameMode))
    (:then
      (Default|AddScore _asgmb_in_game (Utilities|Select :Index _ecollectibletype :NewEnumerator0 100 :NewEnumerator1 250 :NewEnumerator2 500))
      (Default|AddCoins _asgmb_in_game (Utilities|Select :Index _ecollectibletype :NewEnumerator0 1 :NewEnumerator1 5 :NewEnumerator2 10)))
    (:CastFailed
      _))
  (Audio|PlaySound2D (Utilities|Select :Index _ecollectibletype :NewEnumerator0 "/Game/Assets/Audio/Collectible/SC_GetCoins_Cue.SC_GetCoins_Cue" :NewEnumerator1 "/Game/Assets/Audio/Collectible/SC_GetCoins_Cue.SC_GetCoins_Cue" :NewEnumerator2 "/Game/Assets/Audio/Collectible/SC_GetRuby_Cue.SC_GetRuby_Cue") 1.0 1.0 0.0 0 0)
  (Default|PlayFeedback (Variables|Default|GetAs%20BP%20Player) "NewEnumerator3")
  (Actor|DestroyActor))

(fn ConstructionScript
  (Components|StaticMesh|SetStaticMesh (Variables|Default|GetStaticMesh) (Utilities|Select :Index (Variables|Default|GetECollectibleType) :NewEnumerator0 "/Game/Assets/Models/Collectible/Coins/Coin_Coin1.Coin_Coin1" :NewEnumerator1 "/Game/Assets/Models/Collectible/Coins/Coin_CoinStar.Coin_CoinStar" :NewEnumerator2 "/Game/Assets/Models/Collectible/Ruby/Ruby.Ruby")))