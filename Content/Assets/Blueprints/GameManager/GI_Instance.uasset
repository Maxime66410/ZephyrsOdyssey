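; Game instance that tracks the current level and persists per-level progress across sessions.
; On Init it loads the save slot, or creates a BP_SaveGame seeded with default records for every level in ListLevel.
; SaveLevel finds the level's record by name, keeps the highest score and stars and the lowest completion time, derived from the level's time minus the passed value, then writes to the slot.
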(event EventInit
  (Savedata|LoadData))

(fn SetLevelGame
  (params (Levels :type Integer))
  (Variables|Level|SetCurrentLevel (Utilities|Array|Get(acopy) (Variables|/Game/Assets/Blueprints/GamePlay/Menu/Enum/Data/Source/PDA_LevelSelectList.PDA_LevelSelectList_C|GetList (Variables|Level|GetListLevel)) Levels)))

(fn GetLevelName
  (bind _currentlevel (Variables|Level|GetCurrentLevel)
    (:then
      (LocalVariables|SetNamePut (Variables|/Game/Assets/Blueprints/GamePlay/Menu/Enum/Data/Source/PDA_LevelSelect.PDA_LevelSelect_C|GetName _currentlevel))
      (return (LocalVariables|GetNamePut)))
    (:else)))

(fn GetLevelTime
  (bind _currentlevel (Variables|Level|GetCurrentLevel)
    (:then
      (LocalVariables|SetTimePut (Variables|/Game/Assets/Blueprints/GamePlay/Menu/Enum/Data/Source/PDA_LevelSelect.PDA_LevelSelect_C|GetTime _currentlevel))
      (return (LocalVariables|GetTimePut)))
    (:else)))

(fn LoadData
  (bind _returnvalue (SaveGame|DoesSaveGameExist (Variables|Default|GetSlot%20Name)))
  (if _returnvalue
    (bind _returnvalue_2 (SaveGame|LoadGamefromSlot (Variables|Default|GetSlot%20Name)))
    (bind _asbp_save_game (Utilities|Casting|CastToBP_SaveGame _returnvalue_2))
    (Variables|Default|SetAs%20BP%20Save%20Game _asbp_save_game)
    (else
      (bind _returnvalue_3 (SaveGame|CreateSaveGameObject "/Game/Assets/Blueprints/Data/BP_SaveGame.BP_SaveGame_C"))
      (Variables|Default|SetAs%20BP%20Save%20Game _returnvalue_3)
      (Savedata|InitDataSaveFiles))))

(fn SaveGame
  (Variables|Default|GetAs%20BP%20Save%20Game
    (:then
      (SaveGame|SaveGametoSlot (Variables|Default|GetAs%20BP%20Save%20Game) (Variables|Default|GetSlot%20Name)))
    (:else)))

(fn InitDataSaveFiles
  (Variables|Default|GetAs%20BP%20Save%20Game
    (:then
      (for _array_element (Variables|/Game/Assets/Blueprints/GamePlay/Menu/Enum/Data/Source/PDA_LevelSelectList.PDA_LevelSelectList_C|GetList (Variables|Level|GetListLevel))
        (Utilities|Array|Add (Variables|/Game/Assets/Blueprints/Data/BP_SaveGame.BP_SaveGame_C|GetListLevel (Variables|Default|GetAs%20BP%20Save%20Game)) (Utilities|Struct|MakeST_LevelData (Variables|/Game/Assets/Blueprints/GamePlay/Menu/Enum/Data/Source/PDA_LevelSelect.PDA_LevelSelect_C|GetName _array_element) 0 999.0 0)))
      (Savedata|SaveGame))
    (:else)))

(fn SaveLevel
  (params (LevelName :type Name) (BestScore :type Integer) (BestTime :type Float%20%28double-precision%29) (Star :type Byte))
  (LocalVariables|SetLocalName LevelName)
  (LocalVariables|SetLocalScore BestScore)
  (LocalVariables|SetLocalTime BestTime)
  (LocalVariables|SetLocalStar Star)
  (bind _as_bp_save_game (Variables|Default|GetAs%20BP%20Save%20Game)
    (:then
      (bind (_array_element _array_index) (Utilities|Array|ForEachLoopwithBreak (Variables|/Game/Assets/Blueprints/Data/BP_SaveGame.BP_SaveGame_C|GetListLevel _as_bp_save_game) :!label _label)
        (:LoopBody
          (if (== (.name _array_element) (LocalVariables|GetLocalName))
            (LocalVariables|SetGoodIndexToSave _array_index)
            (if (< (LocalVariables|GetLocalScore) (.bestscore _array_element))
              (LocalVariables|SetLocalScore (.bestscore _array_element)))
            (if (> (- (Variables|/Game/Assets/Blueprints/GamePlay/Menu/Enum/Data/Source/PDA_LevelSelect.PDA_LevelSelect_C|GetTime (Variables|Level|GetCurrentLevel)) (LocalVariables|GetLocalTime)) (.besttime _array_element))
              (LocalVariables|SetLocalTime (.besttime _array_element))
              (else
                (LocalVariables|SetLocalTime (- (Variables|/Game/Assets/Blueprints/GamePlay/Menu/Enum/Data/Source/PDA_LevelSelect.PDA_LevelSelect_C|GetTime (Variables|Level|GetCurrentLevel)) (LocalVariables|GetLocalTime)))))
            (if (< (LocalVariables|GetLocalStar) (.star _array_element))
              (LocalVariables|SetLocalStar (.star _array_element)))
            (Utilities|Array|SetArrayElem (Variables|/Game/Assets/Blueprints/Data/BP_SaveGame.BP_SaveGame_C|GetListLevel (Variables|Default|GetAs%20BP%20Save%20Game)) (LocalVariables|GetGoodIndexToSave) (Utilities|Struct|MakeST_LevelData (LocalVariables|GetLocalName) (LocalVariables|GetLocalScore) (LocalVariables|GetLocalTime) (LocalVariables|GetLocalStar)))
            (goto _label Break)))
        (:Completed
          (Savedata|SaveGame))))
    (:else)))