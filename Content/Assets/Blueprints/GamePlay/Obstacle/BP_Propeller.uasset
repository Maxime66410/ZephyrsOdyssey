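; BP_Propeller is an obstacle whose spinning propeller repeatedly launches the player along its arrow direction while they stay inside its box collider.
; A fast looping timer spins BaseTop on yaw, with speed scaled by PowerJump.
; Box overlap starts a looping launch timer, overriding only Z velocity, and end overlap clears it.
; The construction script colors the arrow by PowerJump strength tier.
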(event OnComponentBeginOverlap(Box)
  (params (OverlappedComponent :type Primitive%20Component%20Object%20Reference) (OtherActor :type Actor%20Object%20Reference) (OtherComp :type Primitive%20Component%20Object%20Reference) (OtherBodyIndex :type Integer) (bFromSweep :type Boolean) (SweepResult :type Hit%20Result%20Structure%20%28by%20ref%29))
  ;[0.9231 1 0.04473] Box Collider
  (bind _asbp_player (Utilities|Casting|CastToBP_Player OtherActor))
  (Variables|Default|GetREFPlayer
    (:then
      _)
    (:else
      (Variables|Default|SetREFPlayer _asbp_player)))
  (bind _returnvalue (Utilities|Time|SetTimerbyEvent (EventDispatchers|CreateEvent :!event Custom|PropulsePlayer) 0.1 true))
  (Variables|Default|SetEvent _returnvalue))

(event OnComponentEndOverlap(Box)
  (params (OverlappedComponent :type Primitive%20Component%20Object%20Reference) (OtherActor :type Actor%20Object%20Reference) (OtherComp :type Primitive%20Component%20Object%20Reference) (OtherBodyIndex :type Integer))
  ;[0.9231 1 0.04473] Box Collider
  (Utilities|Casting|CastToBP_Player OtherActor)
  (Utilities|Time|ClearandInvalidateTimerbyHandle (Variables|Default|GetEvent)))

(event Custom|PropulsePlayer
  ;[0.205 0.9303 1] Propulse Player
  (Variables|Default|GetREFPlayer
    (:then
      (Character|LaunchCharacter (Variables|Default|GetREFPlayer) (* (Math|Vector|GetForwardVector (Variables|Default|GetArrow)) (Variables|Default|GetPowerJump)) false true))
    (:else)))

(event Custom|RotatePropeller
  (bind _basetop (Variables|Default|GetBaseTop))
  (bind _relativerotation (Variables|/Script/Engine.SceneComponent|GetRelativeRotation _basetop))
  ;[1 0.4983 0.9027] Rotate Propeller
  (Transformation|SetRelativeRotation _basetop (Math|Rotator|MakeRotator (.roll _relativerotation) (.pitch _relativerotation) (+ (.yaw _relativerotation) (/ (Variables|Default|GetPowerJump) 1e+02))) false false))

(event EventBeginPlay
  ;[0.1302 0.1302 0.1302] Start Engine
  (Utilities|Time|SetTimerbyEvent (EventDispatchers|CreateEvent :!event Custom|RotatePropeller) 0.01 true))

(fn ConstructionScript
  (bind _powerjump (Variables|Default|GetPowerJump))
  (if (<= (Variables|Default|GetPowerJump) 2.5e+02)
    (Components|Arrow|SetArrowColor(LinearColor) (Variables|Default|GetArrow) (Utilities|Struct|MakeLinearColor 0.0 0.0 1.0 1.0))
    (elif (and (> _powerjump 251.0) (<= _powerjump 1e+03))
      (Components|Arrow|SetArrowColor(LinearColor) (Variables|Default|GetArrow) (Utilities|Struct|MakeLinearColor 0.0 1.0 0.0 1.0))
      (else
        (Components|Arrow|SetArrowColor(LinearColor) (Variables|Default|GetArrow) (Utilities|Struct|MakeLinearColor 1.0 0.0 0.0 1.0))))))