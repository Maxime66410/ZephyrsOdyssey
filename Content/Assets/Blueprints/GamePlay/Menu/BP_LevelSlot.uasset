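; BP_LevelSlot is a level-select pedestal that shows a rotating mesh and name widget for one level from a data list.
; Entering the detail box stops the spin, eases rotation to zero and scales up mesh and widget; leaving resumes the spin and shrinks them.
; These animations run on looping function timers instead of Tick.
; Entering the inner box stores the level index in GI_Instance and opens MAP_Loading.
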(event OnComponentBeginOverlap(BoxShowLevelDetail)
  (params (OverlappedComponent :type Primitive%20Component%20Object%20Reference) (OtherActor :type Actor%20Object%20Reference) (OtherComp :type Primitive%20Component%20Object%20Reference) (OtherBodyIndex :type Integer) (bFromSweep :type Boolean) (SweepResult :type Hit%20Result%20Structure%20%28by%20ref%29))
  ;[1 0.09369 0.1036] Player Enter To Focus Level
  (Utilities|Casting|CastToBP_Player OtherActor)
  (Variables|Default|SetIsBox true)
  (bind _returnvalue (Utilities|Time|SetTimerbyFunctionName 0 "ScaleLevelMesh" 0.01 true))
  (Variables|Event|SetEvent_ScaleUpdate _returnvalue)
  (bind _returnvalue_2 (Utilities|Time|SetTimerbyFunctionName 0 "ResetRotationMesh" 0.01 true))
  (Variables|Event|SetEvent_ResetRotationMesh _returnvalue_2)
  (Utilities|Time|ClearandInvalidateTimerbyHandle (Variables|Event|GetEvent_UpdateRotateMesh))
  (Rendering|SetVisibility (Variables|Default|GetWidgetLevel) true false))

(event OnComponentEndOverlap(BoxShowLevelDetail)
  (params (OverlappedComponent :type Primitive%20Component%20Object%20Reference) (OtherActor :type Actor%20Object%20Reference) (OtherComp :type Primitive%20Component%20Object%20Reference) (OtherBodyIndex :type Integer))
  ;[1 0.7825 0] Player Exit
  (Utilities|Casting|CastToBP_Player OtherActor)
  (Variables|Default|SetIsBox false)
  (bind _returnvalue (Utilities|Time|SetTimerbyFunctionName 0 "UpdateRotateMesh" 0.01 true))
  (Variables|Event|SetEvent_UpdateRotateMesh _returnvalue))

(event OnComponentBeginOverlap(BoxEnterLevel)
  (params (OverlappedComponent :type Primitive%20Component%20Object%20Reference) (OtherActor :type Actor%20Object%20Reference) (OtherComp :type Primitive%20Component%20Object%20Reference) (OtherBodyIndex :type Integer) (bFromSweep :type Boolean) (SweepResult :type Hit%20Result%20Structure%20%28by%20ref%29))
  ;[0.01916 1 0] Player Confirm Select Levels
  (Utilities|Casting|CastToBP_Player OtherActor)
  (Setup|SetupLinkLevelsInstance)
  (Game|OpenLevel(byObjectReference) "/Game/Assets/Map/MAP_Loading.MAP_Loading"))

(event EventBeginPlay
  (bind _returnvalue (Utilities|Time|SetTimerbyFunctionName 0 "UpdateRotateMesh" 0.01 true))
  (Variables|Event|SetEvent_UpdateRotateMesh _returnvalue)
  (Setup|SetupUI))

(fn ConstructionScript
  (Components|StaticMesh|SetStaticMesh (Variables|Default|GetLevel) (Variables|/Game/Assets/Blueprints/GamePlay/Menu/Enum/Data/Source/PDA_LevelSelect.PDA_LevelSelect_C|GetMesh (Utilities|Array|Get(acopy) (Variables|/Game/Assets/Blueprints/GamePlay/Menu/Enum/Data/Source/PDA_LevelSelectList.PDA_LevelSelectList_C|GetList (Variables|Default|GetData)) (Math|Conversions|ToInteger(Byte) (Variables|Default|GetLevels))))))

(fn ScaleLevelMesh
  (bind _level (Variables|Default|GetLevel))
  (bind _widgetlevel (Variables|Default|GetWidgetLevel))
  (bind _relativescale3d (Variables|/Script/Engine.SceneComponent|GetRelativeScale3D _level))
  (Transformation|SetRelativeScale3D _level (Math|Interpolation|VInterpTo _relativescale3d (select (Variables|Default|GetIsBox) "1.200000,1.200000,1.200000" "1.000000,1.000000,1.000000") (Utilities|Time|GetWorldDeltaSeconds) 5.0))
  (Transformation|SetRelativeScale3D _widgetlevel (Math|Interpolation|VInterpTo (Variables|/Script/Engine.SceneComponent|GetRelativeScale3D _widgetlevel) (select (Variables|Default|GetIsBox) "0.750000,0.750000,0.750000" "0, 0, 0") (Utilities|Time|GetWorldDeltaSeconds) 5.0))
  (if (< (Math|Vector|Distance(Vector) _relativescale3d "1.000000,1.000000,1.000000") 0.002)
    (Rendering|SetVisibility (Variables|Default|GetWidgetLevel) false false)
    (Utilities|Time|ClearandInvalidateTimerbyHandle (Variables|Event|GetEvent_ScaleUpdate))))

(fn UpdateRotateMesh
  (Transformation|AddLocalRotation (Variables|Default|GetLevel) (Math|Rotator|MakeRotator 0.0 0.0 0.1) false false))

(fn ResetRotationMesh
  (bind _level (Variables|Default|GetLevel))
  (bind _relativerotation (Variables|/Script/Engine.SceneComponent|GetRelativeRotation _level))
  (Transformation|SetRelativeRotation _level (Math|Interpolation|RInterpTo _relativerotation "0, 0, 0" (Utilities|Time|GetWorldDeltaSeconds) 5.0) false false)
  (if (Utilities|Operators|EqualEqual :A _relativerotation :ErrorTolerance 0.1)
    (Utilities|Time|ClearandInvalidateTimerbyHandle (Variables|Event|GetEvent_ResetRotationMesh))))

(fn SetupUI
  (bind _returnvalue (UserInterface|CreateWidget "/Game/Assets/Blueprints/UI/Level/UW_Level.UW_Level_C"))
  (UserInterface|SetWidget (Variables|Default|GetWidgetLevel) _returnvalue)
  (Default|SetupInformation _returnvalue (Utilities|Text|ToText(Name) (Variables|/Game/Assets/Blueprints/GamePlay/Menu/Enum/Data/Source/PDA_LevelSelect.PDA_LevelSelect_C|GetName (Utilities|Array|Get(acopy) (Variables|/Game/Assets/Blueprints/GamePlay/Menu/Enum/Data/Source/PDA_LevelSelectList.PDA_LevelSelectList_C|GetList (Variables|Default|GetData)) (Math|Conversions|ToInteger(Byte) (Variables|Default|GetLevels)))))))

(fn SetupLinkLevelsInstance
  (bind _asgi_instance (Utilities|Casting|CastToGI_Instance (Game|GetGameInstance)))
  (bind _output_get (Variables|REF|SetAs%20GI%20Instance _asgi_instance))
  (Default|SetLevelGame _output_get (Math|Conversions|ToInteger(Byte) (Variables|Default|GetLevels))))