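; In-game game manager that runs a level's countdown, tracks score and coins, and handles end of game.
; BeginPlay creates the UW_InGame HUD and starts a one-second looping timer from GI_Instance's level time, which pausing clears or restarts.
; Add functions update values and HUD, with coins also adding score.
; Timeout or EndGame totals score, coins and remaining time, rates stars and win state against thresholds, freezes the player and saves through GI_Instance.
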(event Custom|EndGame
  (Utilities|Time|ClearandInvalidateTimerbyHandle (Variables|Event|GetEvent_SequenceTimer))
  (GamePlay|CheckScore))

(event EventBeginPlay
  (Setup|GetPlayer)
  (Setup|GetInstance)
  (Setup|SetupUI)
  (bind _returnvalue (Utilities|Time|SetTimerbyFunctionName 0 "SequenceTimer" 1.0 true))
  (Variables|Event|SetEvent_SequenceTimer _returnvalue))

(fn ConstructionScript)

(fn GetPlayer
  (bind _returnvalue (Actor|GetActorOfClass "/Game/Assets/Blueprints/Player/BP_Player.BP_Player_C"))
  (Variables|REF|SetAs%20Player _returnvalue))

(fn SetupUI
  (Utilities|FlowControl|Sequence
    (:then_0
      ;[1 0.7701 0] Setup UI on ViewPort
      (bind _returnvalue (UserInterface|CreateWidget "/Game/Assets/Blueprints/UI/UW_InGame.UW_InGame_C" (Pawn|GetLocalViewingPlayerController (Variables|REF|GetAs%20Player))))
      (bind _output_get (Variables|REF|SetAs%20UIBase _returnvalue))
      (UserInterface|Viewport|AddtoViewport _output_get 0)
      (Default|AddUIinGame (Variables|REF|GetAs%20Player) (Variables|REF|GetAs%20UIBase))
      (Default|GetPlayer (Variables|REF|GetAs%20UIBase) (Variables|REF|GetAs%20Player)))
    (:then_1
      ;[1 0.1394 0] Get Time Level
      (Variables|GamePlay|SetCurrentTime (Default|GetLevelTime (Variables|REF|GetAs%20GI%20Instance))))
    (:then_2
      ;[0 0.1341 1] Init Value on UI
      (Default|UpdateScoring (Variables|REF|GetAs%20UIBase) (Variables|GamePlay|GetScore))
      (Default|UpdateCoins (Variables|REF|GetAs%20UIBase) (Variables|GamePlay|GetCoins))
      (Default|UpdateTime (Variables|REF|GetAs%20UIBase) (Variables|GamePlay|GetCurrentTime)))))

(fn GetInstance
  (bind _asgi_instance (Utilities|Casting|CastToGI_Instance (Game|GetGameInstance)))
  (Variables|REF|SetAs%20GI%20Instance _asgi_instance))

(fn SequenceTimer
  (bind _currenttime (Variables|GamePlay|GetCurrentTime))
  (if (> _currenttime 0.0)
    (Math|Float|DecrementFloat _currenttime
      (:%20%20
        (bind _as_uibase (Variables|REF|GetAs%20UIBase)
          (:then
            (Default|UpdateTime _as_uibase (Variables|GamePlay|GetCurrentTime)))
          (:else))))
    (else
      (GamePlay|CheckScore)
      (Audio|PlaySound2D "/Game/Assets/Audio/Collectible/SC_Circus-lose-2030_Cue.SC_Circus-lose-2030_Cue" 1.0 1.0 0.0 0 0)
      (Utilities|Time|ClearandInvalidateTimerbyHandle (Variables|Event|GetEvent_SequenceTimer)))))

(fn AddTime
  (params (ToAdd :type Float%20%28double-precision%29))
  (Variables|GamePlay|SetCurrentTime (+ (Variables|GamePlay|GetCurrentTime) ToAdd))
  (bind _as_uibase (Variables|REF|GetAs%20UIBase)
    (:then
      (Default|UpdateTime _as_uibase (Variables|GamePlay|GetCurrentTime)))
    (:else)))

(fn AddScore
  (params (ToAdd :type Integer))
  (Variables|GamePlay|SetScore (+ (Variables|GamePlay|GetScore) ToAdd))
  (bind _as_uibase (Variables|REF|GetAs%20UIBase)
    (:then
      (Default|UpdateScoring _as_uibase (Variables|GamePlay|GetScore)))
    (:else)))

(fn AddCoins
  (params (AddCoins :type Integer))
  (Variables|GamePlay|SetCoins (+ (Variables|GamePlay|GetCoins) AddCoins))
  (GamePlay|AddScore 50)
  (bind _as_uibase (Variables|REF|GetAs%20UIBase)
    (:then
      (Default|UpdateCoins _as_uibase (Variables|GamePlay|GetCoins)))
    (:else)))

(fn SetPause
  (params (Pause? :type Boolean))
  (if Pause?
    (if (Utilities|Time|IsTimerActivebyHandle (Variables|Event|GetEvent_SequenceTimer))
      (Utilities|Time|ClearandInvalidateTimerbyHandle (Variables|Event|GetEvent_SequenceTimer)))
    (elif (not (Utilities|Time|IsTimerActivebyHandle (Variables|Event|GetEvent_SequenceTimer)))
      (bind _returnvalue (Utilities|Time|SetTimerbyFunctionName 0 "SequenceTimer" 1.0 true))
      (Variables|Event|SetEvent_SequenceTimer _returnvalue))))

(fn CheckScore
  ;[1 0.3634 0] Setup Final Score
  (Default|UpdateFinalScoring (Variables|REF|GetAs%20UIBase) (+ (Variables|GamePlay|GetScore) (Variables|GamePlay|GetCoins) (Math|Float|Round (Variables|GamePlay|GetCurrentTime))) (Variables|GamePlay|GetCurrentTime))
  ;[0 1 0.7155] Create fake local Score
  (LocalVariables|SetLocalScore (+ (Variables|GamePlay|GetScore) (Variables|GamePlay|GetCoins) (Math|Float|Round (Variables|GamePlay|GetCurrentTime))))
  ;[0.9673 1 0] Check Score Star
  (bind _array_element (Utilities|Array|ForEachLoopwithBreak (LocalVariables|GetGetStar) :!label _label)
    (:LoopBody
      (if (> _array_element (LocalVariables|GetLocalScore))
        (LocalVariables|SetIsWin? false)
        (goto _label Break)
        (else
          (Math|Integer|IncrementInt (LocalVariables|GetCurrentStar)))))
    (:Completed
      ;[1 0.09911 0] Set Star Score & Show Score
      (Default|SetStarLogic (Variables|REF|GetAs%20UIBase) (- (LocalVariables|GetCurrentStar) 1))
      (Default|SetEndGameState (Variables|REF|GetAs%20UIBase) (select (LocalVariables|GetIsWin?) "NewEnumerator0" "NewEnumerator1"))
      ;[0.7859 1 0] Freeze Players
      (Default|ReactivateInputMovement (Variables|REF|GetAs%20Player) true)
      ;[1 0 0.03671] Save Data
      (bind _as_gi_instance (Variables|REF|GetAs%20GI%20Instance)
        (:then
          (Default|SaveLevel _as_gi_instance (Variables|/Game/Assets/Blueprints/GamePlay/Menu/Enum/Data/Source/PDA_LevelSelect.PDA_LevelSelect_C|GetName (Variables|/Game/Assets/Blueprints/GameManager/GI_Instance.GI_Instance_C|GetCurrentLevel _as_gi_instance)) (LocalVariables|GetLocalScore) (Variables|GamePlay|GetCurrentTime) (Math|Conversions|ToByte(Integer) (LocalVariables|GetCurrentStar))))
        (:else)))))