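; BP_LevelShow is a menu actor that displays a static mesh matching the currently selected level.
; On BeginPlay it casts the game instance to GI_Instance and searches its level list for the current level.
; The matching index selects one of three level meshes to set on its StaticMesh component.
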(event EventBeginPlay
  (bind _asgi_instance (Utilities|Casting|CastToGI_Instance (Game|GetGameInstance)))
  (bind _output_get (Variables|Default|SetAs%20GI%20Instance _asgi_instance))
  (bind (_array_element _array_index) (Utilities|Array|ForEachLoopwithBreak (Variables|/Game/Assets/Blueprints/GamePlay/Menu/Enum/Data/Source/PDA_LevelSelectList.PDA_LevelSelectList_C|GetList (Variables|/Game/Assets/Blueprints/GameManager/GI_Instance.GI_Instance_C|GetListLevel _output_get)) :!label _label)
    (:LoopBody
      (if (== _array_element (Variables|/Game/Assets/Blueprints/GameManager/GI_Instance.GI_Instance_C|GetCurrentLevel _output_get))
        (Components|StaticMesh|SetStaticMesh (Variables|Default|GetStaticMesh) (Utilities|Select :Index _array_index :Option%200 "/Game/Assets/Models/MainMenu/Level/Level1.Level1" :Option%201 "/Game/Assets/Models/MainMenu/Level/Level2.Level2" :Option%202 "/Game/Assets/Models/MainMenu/Level/Level3.Level3"))
        (goto _label Break)))))

(fn ConstructionScript)