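; BP_FallPlank is a plank platform obstacle that falls through physics simulation and has logic to respawn.
; Depending on its Event setting, a player hit starts a delay timer, or leaving the box overlap drops it immediately.
; Physics activation starts a respawn timer; Respawn stops simulation and applies transforms saved at BeginPlay, captured in world space but restored as relative.
; The construction script fits mesh and trigger box to the Normal or Large design.
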(event OnComponentHit(Planche)
  (params (HitComponent :type Primitive%20Component%20Object%20Reference) (OtherActor :type Actor%20Object%20Reference) (OtherComp :type Primitive%20Component%20Object%20Reference) (NormalImpulse :type Vector :default "0, 0, 0") (Hit :type Hit%20Result%20Structure%20%28by%20ref%29))
  ;[0.6454 1 0.1314] Activate On Hit
  (Utilities|Casting|CastToBP_Player OtherActor)
  (if (Utilities|Enum|Equal(Enum) (Variables|Default|GetEvent) "NewEnumerator0")
    (if (not (Variables|Default|GetIsDestroy))
      (Utilities|Time|SetTimerbyEvent (EventDispatchers|CreateEvent :!event Custom|ActivatePhysics) (Variables|Default|GetDelayToFall))
      (Variables|Default|SetIsDestroy true))))

(event OnComponentEndOverlap(Box)
  (params (OverlappedComponent :type Primitive%20Component%20Object%20Reference) (OtherActor :type Actor%20Object%20Reference) (OtherComp :type Primitive%20Component%20Object%20Reference) (OtherBodyIndex :type Integer))
  ;[0.4922 0.3904 1] Activate On Jump
  (Utilities|Casting|CastToBP_Player OtherActor)
  (if (Utilities|Enum|Equal(Enum) (Variables|Default|GetEvent) "NewEnumerator1")
    (if (not (Variables|Default|GetIsDestroy))
      (CallFunction|ActivatePhysics)
      (Variables|Default|SetIsDestroy true))))

(event Custom|ActivatePhysics
  ;[1 0.1707 0.6226] Enable Physics
  (Physics|SetSimulatePhysics (Variables|Default|GetPlanche) true)
  (Physics|SetSimulatePhysics (Variables|Default|GetStructure) true)
  (Utilities|Time|SetTimerbyEvent (EventDispatchers|CreateEvent :!event Custom|Respawn) 5.0))

(event Custom|Respawn
  (bind _transformsave (Variables|Default|GetTransformSave))
  (bind _transformsave_2 (Variables|Default|GetTransformSave))
  (bind _output (Utilities|Array|Get(acopy) _transformsave 1))
  (bind _output_2 (Utilities|Array|Get(acopy) _transformsave_2))
  ;[0.1188 0.1619 1] Respawn platforme
  (Utilities|FlowControl|Sequence
    (:then_0
      (Variables|Default|SetIsDestroy false))
    (:then_1
      (Physics|SetSimulatePhysics (Variables|Default|GetStructure) false)
      (Physics|SetSimulatePhysics (Variables|Default|GetPlanche) false))
    (:then_2
      (Transformation|SetRelativeLocationAndRotation (Variables|Default|GetStructure) (.location _output_2) (.rotation _output_2) false true)
      (Transformation|SetRelativeLocationAndRotation (Variables|Default|GetPlanche) (.location _output) (.rotation _output) false true))))

(event EventBeginPlay
  (CallFunction|GetPosRot))

(fn ConstructionScript
  (bind _box (Variables|Default|GetBox))
  (bind _plank_design (Variables|Default|GetPlank%20Design))
  (Utilities|FlowControl|Sequence
    (:then_0
      ;[1 0.117 0.3694] Update mesh Type
      (Components|StaticMesh|SetStaticMesh (Variables|Default|GetPlanche) (Utilities|Select :Index (Variables|Default|GetPlank%20Design) :NewEnumerator0 "/Game/Assets/Models/Props/Planche/LittlePlanche.LittlePlanche" :NewEnumerator1 "/Game/Assets/Models/Props/Planche/Planche.Planche")))
    (:then_1
      ;[1 0.9495 0.08993] Update box Collision
      (Components|Box|SetBoxExtent _box (Utilities|Select :Index _plank_design :NewEnumerator0 "212.308074,200.547917,15.000000" :NewEnumerator1 "306.590914,200.547917,15.000000") true)
      (Transformation|SetRelativeLocation _box (Utilities|Select :Index _plank_design :NewEnumerator0 "-196.805503,0.000000,13.100953" :NewEnumerator1 "-301.231035,0.000000,13.100953") false false))))

(fn GetPosRot
  (bind _transformsave (Variables|Default|GetTransformSave))
  (bind _structure (Variables|Default|GetStructure))
  (bind _planche (Variables|Default|GetPlanche))
  (Utilities|Array|Add _transformsave (Math|Transform|MakeTransform (Transformation|GetWorldLocation _structure) (Transformation|GetWorldRotation _structure) "1.000000,1.000000,1.000000"))
  (Utilities|Array|Add _transformsave (Math|Transform|MakeTransform (Transformation|GetWorldLocation _planche) (Transformation|GetWorldRotation _planche) "1.000000,1.000000,1.000000")))