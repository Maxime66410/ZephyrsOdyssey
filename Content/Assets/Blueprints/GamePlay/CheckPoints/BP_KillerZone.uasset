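; BP_KillerZone is a kill volume that respawns the player at a spawn reference when its box is overlapped.
; The first overlap by a BP_Player caches it; later overlaps reuse that cached player without checking the overlapping actor.
; CheckPlayer zeroes the player's velocity and teleports it to REFSpawn's location, using the zone's own rotation.
; SetNewSpawn lets the respawn point be replaced.
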(event OnComponentBeginOverlap(Box)
  (params (OverlappedComponent :type Primitive%20Component%20Object%20Reference) (OtherActor :type Actor%20Object%20Reference) (OtherComp :type Primitive%20Component%20Object%20Reference) (OtherBodyIndex :type Integer) (bFromSweep :type Boolean) (SweepResult :type Hit%20Result%20Structure%20%28by%20ref%29))
  ;[0.2917 0.05613 0.0823] Respawn Player
  (bind _as_bp_player (Variables|Default|GetAs%20BP%20Player)
    (:then
      (Variables|/Script/Engine.MovementComponent|SetVelocity (Variables|/Script/Engine.Character|GetCharacterMovement _as_bp_player) "0, 0, 0")
      (Transformation|Teleport (Variables|Default|GetAs%20BP%20Player) (Transformation|GetActorLocation (Variables|REF|GetREFSpawn)) (Transformation|GetActorRotation)))
    (:else
      (bind _asbp_player (Utilities|Casting|CastToBP_Player OtherActor))
      (Variables|Default|SetAs%20BP%20Player _asbp_player)
      (CallFunction|CheckPlayer))))

(event Custom|CheckPlayer
  ;[0.2917 0.05613 0.0823] Respawn Player
  (bind _as_bp_player (Variables|Default|GetAs%20BP%20Player)
    (:then
      (Variables|/Script/Engine.MovementComponent|SetVelocity (Variables|/Script/Engine.Character|GetCharacterMovement _as_bp_player) "0, 0, 0")
      (Transformation|Teleport (Variables|Default|GetAs%20BP%20Player) (Transformation|GetActorLocation (Variables|REF|GetREFSpawn)) (Transformation|GetActorRotation)))
    (:else
      (bind _asbp_player (Utilities|Casting|CastToBP_Player (stale OnComponentBeginOverlap(Box) OtherActor)))
      (Variables|Default|SetAs%20BP%20Player _asbp_player)
      (CallFunction|CheckPlayer))))

(fn ConstructionScript)

(fn SetNewSpawn
  (params (REFSpawn :type BP%20Check%20Points%20Object%20Reference))
  (Variables|REF|SetREFSpawn REFSpawn))