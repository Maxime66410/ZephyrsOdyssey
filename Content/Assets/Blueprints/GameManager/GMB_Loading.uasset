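; GMB_Loading is the loading-screen game mode that shows information about the selected level, then opens it.
; On BeginPlay it creates the UW_Loading widget, reads CurrentLevel from GI_Instance and passes the level's name and time to the widget.
; After a fixed short delay it opens that level by object reference, with no real load tracking.
; An unconnected stream-level load remains, noted as working only with sublevels.
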(event EventBeginPlay
  (Utilities|FlowControl|Sequence
    (:then_0
      (CallFunction|SetupUI))
    (:then_1
      (CallFunction|PreparingInformation))
    (:then_2
      (CallFunction|SetupInformationUI))
    (:then_3
      (Utilities|FlowControl|Delay 2.0)
      (Game|OpenLevel(byObjectReference) (Variables|Default|GetLocalLevel)))))

(fn ConstructionScript)

(fn SetupUI
  (bind _returnvalue (UserInterface|CreateWidget "/Game/Assets/Blueprints/UI/UW_Loading.UW_Loading_C" (Game|GetPlayerController 0)))
  (bind _output_get (Variables|Default|Setas%20Loading%20UI _returnvalue))
  (UserInterface|Viewport|AddtoViewport _output_get 0))

(fn PreparingInformation
  (bind _asgi_instance (Utilities|Casting|CastToGI_Instance (Game|GetGameInstance)))
  (Variables|Default|SetAs%20GI%20Instance _asgi_instance)
  (Variables|Default|SetLocalName (Variables|/Game/Assets/Blueprints/GamePlay/Menu/Enum/Data/Source/PDA_LevelSelect.PDA_LevelSelect_C|GetName (Variables|/Game/Assets/Blueprints/GameManager/GI_Instance.GI_Instance_C|GetCurrentLevel (Variables|Default|GetAs%20GI%20Instance))))
  (Variables|Default|SetLocalTime (Variables|/Game/Assets/Blueprints/GamePlay/Menu/Enum/Data/Source/PDA_LevelSelect.PDA_LevelSelect_C|GetTime (Variables|/Game/Assets/Blueprints/GameManager/GI_Instance.GI_Instance_C|GetCurrentLevel (Variables|Default|GetAs%20GI%20Instance))))
  (Variables|Default|SetLocalLevel (Variables|/Game/Assets/Blueprints/GamePlay/Menu/Enum/Data/Source/PDA_LevelSelect.PDA_LevelSelect_C|GetLevel (Variables|/Game/Assets/Blueprints/GameManager/GI_Instance.GI_Instance_C|GetCurrentLevel (Variables|Default|GetAs%20GI%20Instance)))))

(fn SetupInformationUI
  (bind _as_loading_ui (Variables|Default|Getas%20Loading%20UI)
    (:then
      (Default|SetInformation _as_loading_ui (Variables|Default|GetLocalTime) (Variables|Default|GetLocalName)))
    (:else)))