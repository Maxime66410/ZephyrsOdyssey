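; Decorative fake boat that travels along a referenced spline path while its two propellers spin.
; A looping timer set on BeginPlay appears to drive the propeller rotation.
; If the spline is valid, a timeline with play rate set from the circuit time lerps distance along it.
; Each update sets position, rotation and a fixed reduced scale, adding a random offset chosen at start.
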(event Custom|Move%20Object
  (bind _splinepath (Variables|Default|GetSplinePath))
  (bind _spline (Variables|/Game/Assets/Blueprints/GamePlay/Decor/Spline/BP_SplinePath.BP_SplinePath_C|GetSpline _splinepath))
  ;[0 0.2809 1] Move Object
  (Components|Timeline|SetPlayRate (Variables|Default|GetMoving%20Object) (/ 1.0 (Variables|Default|GetCircuit%20Time%20%28seconds%29)))
  (bind _move_track (Timeline|Moving%20Object Play)
    (:Update
      (Transformation|SetActorTransform (Math|Transform|MakeTransform (+ (Spline|GetLocationatDistanceAlongSpline _spline (Math|Float|Lerp 0.0 (Spline|GetSplineLength (Variables|/Game/Assets/Blueprints/GamePlay/Decor/Spline/BP_SplinePath.BP_SplinePath_C|GetSpline (Variables|Default|GetSplinePath))) _move_track) "World") (Variables|Default|GetVectorOffSet)) (Spline|GetRotationatDistanceAlongSpline _spline (Math|Float|Lerp 0.0 (Spline|GetSplineLength (Variables|/Game/Assets/Blueprints/GamePlay/Decor/Spline/BP_SplinePath.BP_SplinePath_C|GetSpline (Variables|Default|GetSplinePath))) _move_track) "World") "0.450000,0.450000,0.450000")))))

(event Custom|RotatePropeller
  ;[0.1402 0.7264 1] Rotate Propeller
  (Transformation|AddLocalRotation (Variables|Default|GetHPropeller2) (Math|Rotator|MakeRotator 0.0 (Variables|Default|GetSpeed) 0.0) false false)
  (Transformation|AddLocalRotation (Variables|Default|GetHPropeller) (Math|Rotator|MakeRotator 0.0 (Variables|Default|GetSpeed) 0.0) false false))

(event EventBeginPlay
  (Utilities|Time|SetTimerbyEvent (EventDispatchers|CreateEvent :!event Custom|RotatePropeller) 0.01 true)
  (Variables|Default|GetSplinePath
    (:then
      ;[0 1 0.08618] Random Offset
      (Variables|Default|SetVectorOffSet (Math|Vector|MakeVector (Math|Random|RandomFloatinRange -3e+02 3e+02) (Math|Random|RandomFloatinRange -3e+02 3e+02) (Math|Random|RandomFloatinRange -3e+02 3e+02)))
      ;[1 0 0.3103] Start Move Object
      (CallFunction|MoveObject))
    (:else)))

(fn ConstructionScript)